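; Player controller for Two Left Standing that handles level travel, shared pausing and objective HUD updates in multiplayer.
; Server events ServerTravel to one of four level maps using the TwoLeft game mode.
; Escape asks the server to toggle global pause, which notifies every controller to show or remove a pause widget naming the pausing player and switch input mode.
; A client event pushes objective text to the player HUD widget.
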(event Custom|Server_StartLevel1
  (Development|ExecuteConsoleCommand "ServerTravel Map_Level1?game=/Game/TwoLeftStanding/BP_TwoLeftGameMode.BP_TwoLeftGameMode_C" (Game|GetPlayerController 0)))

(event Custom|Server_ToggleGlobalPause
  (bind _returnvalue (Game|IsGamePaused))
  (bind _returnvalue_2 (not _returnvalue))
  (bind _outactors (Actor|GetAllActorsOfClass "BP_TwoLeftController_C"))
  (for _array_element _outactors
    (CallFunction|ClientTogglePauseUI _array_element _returnvalue_2 self))
  (Game|SetGamePaused _returnvalue_2))

(event Custom|Client_TogglePauseUI
  (params (IsPaused :type Boolean) (PausingPlayer :type Player%20Controller%20Object%20Reference))
  (bind _returnvalue (Game|GetPlayerController 0))
  (bind _returnvalue_2 (Game|GetPlayerController 0))
  (if IsPaused
    (Utilities|IsValid (Variables|Default|GetPauseMenuRef)
      (:Is%20Valid
        (Widget|RemovefromParent (Variables|Default|GetPauseMenuRef)))
      (:Is%20Not%20Valid
        _))
    (bind _returnvalue_3 (UserInterface|CreateWidget "/Game/TwoLeftStanding/UI/WBP_Paused.WBP_Paused_C" 0 PausingPlayer))
    (Variables|Default|SetPauseMenuRef _returnvalue_3)
    (UserInterface|Viewport|AddtoViewport _returnvalue_3 100)
    (Input|SetInputModeGameandUI _returnvalue _returnvalue_3 "DoNotLock" true false)
    (Variables|/Script/Engine.PlayerController|SetbShowMouseCursor _returnvalue true)
    (else
      (Widget|RemovefromParent (Variables|Default|GetPauseMenuRef))
      (Variables|Default|SetPauseMenuRef 0)
      (Input|SetInputModeGameOnly _returnvalue_2 false)
      (Variables|/Script/Engine.PlayerController|SetbShowMouseCursor _returnvalue_2 false))))

(event Custom|Client_UpdateObjectiveUI
  (params (ObjectiveMessage :type Text))
  (bind _foundwidgets (Widget|GetAllWidgetsOfClass "/Game/TwoLeftStanding/UI/WBP_PlayerHUD.WBP_PlayerHUD_C" true))
  (Default|UpdateObjectiveText (Utilities|Array|Get(acopy) _foundwidgets) ObjectiveMessage))

(event Custom|Server_StartLevel2
  (Development|ExecuteConsoleCommand "ServerTravel Map_Level2?game=/Game/TwoLeftStanding/BP_TwoLeftGameMode.BP_TwoLeftGameMode_C" (Game|GetPlayerController 0)))

(event Custom|Server_StartLevel3
  (Development|ExecuteConsoleCommand "ServerTravel Map_Level3?game=/Game/TwoLeftStanding/BP_TwoLeftGameMode.BP_TwoLeftGameMode_C" (Game|GetPlayerController 0)))

(event Custom|Server_StartLevel4
  (Development|ExecuteConsoleCommand "ServerTravel Map_Level4?game=/Game/TwoLeftStanding/BP_TwoLeftGameMode.BP_TwoLeftGameMode_C" (Game|GetPlayerController 0)))

(event EventBeginPlay)

(event EventTick
  (params (DeltaSeconds :type Float%20%28single-precision%29)))

(event Input|KeyboardEvents|Escape
  (params (Key :type Key%20Structure :default "None"))
  (:Pressed
    (CallFunction|ServerToggleGlobalPause)))

(fn ConstructionScript)