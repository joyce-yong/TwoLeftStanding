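; Game instance for TwoLeftStanding that restores the player's audio volume settings when the game starts.
; On Init it activates the user-settings control bus mix, then loads the AudioSettings save slot if one exists.
; Saved master, music and SFX volumes are pushed to their Audio Modulation control buses through short-ramped mix updates.
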(event EventInit
  (Class|AudioModulationStatics|ActivateBusMix "/Game/TwoLeftStanding/Audio/AudioMix/Modulation/ControlBusMix/CBM_UserSettings.CBM_UserSettings")
  (bind _returnvalue (SaveGame|DoesSaveGameExist "AudioSettings"))
  (if _returnvalue
    (bind _returnvalue_2 (SaveGame|LoadGamefromSlot "AudioSettings"))
    (bind _asbp_two_left_save_game (Utilities|Casting|CastToBP_TwoLeftSaveGame _returnvalue_2))
    (Class|AudioModulationStatics|UpdateMix "/Game/TwoLeftStanding/Audio/AudioMix/Modulation/ControlBusMix/CBM_UserSettings.CBM_UserSettings" (Utilities|Array|MakeArray (Utilities|Struct|MakeSoundControlBusMixStage "/Game/TwoLeftStanding/Audio/AudioMix/Modulation/ControlBus/User/CB_User_Master.CB_User_Master" (Utilities|Struct|MakeSoundModulationMixValue (Variables|/Game/TwoLeftStanding/BP_TwoLeftSaveGame.BP_TwoLeftSaveGame_C|GetSaved_MasterVol _asbp_two_left_save_game) 0.05 0.05))))
    (Class|AudioModulationStatics|UpdateMix "/Game/TwoLeftStanding/Audio/AudioMix/Modulation/ControlBusMix/CBM_UserSettings.CBM_UserSettings" (Utilities|Array|MakeArray (Utilities|Struct|MakeSoundControlBusMixStage "/Game/TwoLeftStanding/Audio/AudioMix/Modulation/ControlBus/User/CB_User_Music.CB_User_Music" (Utilities|Struct|MakeSoundModulationMixValue (Variables|/Game/TwoLeftStanding/BP_TwoLeftSaveGame.BP_TwoLeftSaveGame_C|GetSaved_MusicVol _asbp_two_left_save_game) 0.05 0.05))))
    (Class|AudioModulationStatics|UpdateMix "/Game/TwoLeftStanding/Audio/AudioMix/Modulation/ControlBusMix/CBM_UserSettings.CBM_UserSettings" (Utilities|Array|MakeArray (Utilities|Struct|MakeSoundControlBusMixStage "/Game/TwoLeftStanding/Audio/AudioMix/Modulation/ControlBus/User/CB_User_SFX.CB_User_SFX" (Utilities|Struct|MakeSoundModulationMixValue (Variables|/Game/TwoLeftStanding/BP_TwoLeftSaveGame.BP_TwoLeftSaveGame_C|GetSaved_SFXVol _asbp_two_left_save_game) 0.05 0.05))))))