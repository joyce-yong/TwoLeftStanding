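; BP_Fishie is an enemy character with a floating health bar above it.
; Every tick it pushes current and max health into its WBP_EnemyHealthBar widget and rotates the widget component to face the player camera.
; An unconnected death sequence, which never runs, would unpossess AIC_Fishie, disable capsule collision, play the death montage and set a lifespan for delayed removal.
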(event EventTick
  (params (DeltaSeconds :type Float%20%28single-precision%29))
  (bind _health_bar_widget (Variables|Default|GetHealth%20Bar%20Widget))
  (bind _aswbp_enemy_health_bar (Utilities|Casting|CastToWBP_EnemyHealthBar (UserInterface|GetWidget (Variables|Default|GetHealth%20Bar%20Widget))))
  (Default|UpdateHealth _aswbp_enemy_health_bar (Variables|Default|GetCurrentHealth) (Variables|Default|GetMaxHealth))
  (Transformation|SetWorldRotation _health_bar_widget (Math|Rotator|FindLookatRotation (Transformation|GetWorldLocation _health_bar_widget) (Transformation|GetWorldLocation (Variables|/Script/Engine.PlayerCameraManager|GetTransformComponent (Game|GetPlayerCameraManager 0)))) false false))

(fn ConstructionScript)