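; Player character for TwoLeftStanding with two model variants, handling appearance, player UI and the lobby level-select menu.
; The authority assigns ModelIndex 0 to player controller 0's character and 1 otherwise; OnRep applies matching mesh, anim class and gun material.
; The local player gets fade and HUD widgets, a level-failed screen event, and F near BP_LobbyDoor toggles level select.
; Shoot and revive events play model-specific montages.
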(event Custom|Client_ShowLevelFailed
  (bind _returnvalue (Game|GetPlayerController 0))
  (Variables|/Script/Engine.PlayerController|SetbShowMouseCursor _returnvalue true)
  (Input|DisableInput _returnvalue)
  (bind _returnvalue_2 (UserInterface|CreateWidget "/Game/TwoLeftStanding/UI/WBP_LevelFailed.WBP_LevelFailed_C"))
  (UserInterface|Viewport|AddtoViewport _returnvalue_2 0))

(event EventBeginPlay
  (bind _returnvalue (Game|GetPlayerController 0))
  (Utilities|FlowControl|Sequence
    (:then_0
      (Networking|SwitchHasAuthority
        (:Authority
          (if (== (Pawn|GetController) (Game|GetPlayerController 0))
            (Variables|Default|SetModelIndex 0)
            (else
              (Variables|Default|SetModelIndex 1)))
          (CallFunction|UpdateCharacterModel))))
    (:then_1
      (if (Pawn|IsLocallyControlled)
        (Utilities|FlowControl|Delay 0.1)
        (Variables|/Script/Engine.PlayerController|SetbShowMouseCursor _returnvalue false)
        (Input|SetInputModeGameOnly _returnvalue false)
        (bind _returnvalue_2 (UserInterface|CreateWidget "/Game/TwoLeftStanding/UI/WBP_FadeScreen.WBP_FadeScreen_C"))
        (UserInterface|Viewport|AddtoViewport _returnvalue_2 10)
        (bind _foundwidgets (Widget|GetAllWidgetsOfClass "/Game/TwoLeftStanding/UI/WBP_LevelFailed.WBP_LevelFailed_C" true))
        (for _array_element _foundwidgets
          (Widget|RemovefromParent _array_element))
        (bind _foundwidgets_2 (Widget|GetAllWidgetsOfClass "/Game/TwoLeftStanding/UI/WBP_PlayerHUD.WBP_PlayerHUD_C" true))
        (for _array_element_2 _foundwidgets_2
          (Widget|RemovefromParent _array_element_2))
        (bind _returnvalue_3 (UserInterface|CreateWidget "/Game/TwoLeftStanding/UI/WBP_PlayerHUD.WBP_PlayerHUD_C"))
        (UserInterface|Viewport|AddtoViewport _returnvalue_3 10)))))

(event Collision|EventActorBeginOverlap
  (params (OtherActor :type Actor%20Object%20Reference)))

(event EventTick
  (params (DeltaSeconds :type Float%20%28single-precision%29)))

(event EventPlayShootAnimation
  (if (== (Variables|Default|GetModelIndex) 0)
    (Animation|Montage|PlayMontage (Variables|Character|GetMesh) "/Game/TwoLeftStanding/Player/Characters/starlord/AM_Male_Shoot.AM_Male_Shoot")
    (else
      (Animation|Montage|PlayMontage (Variables|Character|GetMesh) "/Game/TwoLeftStanding/Player/Characters/psylocke/AM_Female_Shoot.AM_Female_Shoot"))))

(event EventPlayReviveAnimation
  (if (== (Variables|Default|GetModelIndex) 0)
    (Animation|Montage|PlayMontage (Variables|Character|GetMesh) "/Game/TwoLeftStanding/Player/Characters/starlord/AM_Male_Revive.AM_Male_Revive")
    (else
      (Animation|Montage|PlayMontage (Variables|Character|GetMesh) "/Game/TwoLeftStanding/Player/Characters/psylocke/AM_Female_Revive.AM_Female_Revive"))))

(event EventStopReviveAnimation
  (Animation|Montage|MontageStop (Components|SkeletalMesh|GetAnimInstance (Variables|Character|GetMesh)) 0.0 0))

(event Input|KeyboardEvents|F
  (params (Key :type Key%20Structure :default "None"))
  (bind _returnvalue (Game|GetPlayerController 0))
  (bind _returnvalue_2 (Game|GetPlayerController 0))
  (:Pressed
    (if (> (Utilities|Array|Length (Collision|GetOverlappingActors "/Game/TwoLeftStanding/BP_LobbyDoor.BP_LobbyDoor_C" :!class /Script/Engine.Actor)) 0)
      (if (Variables|Default|GetbIsMenuOpen)
        (Widget|RemovefromParent (Variables|Default|GetLevelSelectUIRef))
        (Variables|Default|SetbIsMenuOpen false)
        (Variables|/Script/Engine.PlayerController|SetbShowMouseCursor _returnvalue false)
        (Input|SetInputModeGameOnly _returnvalue false)
        (bind _foundwidgets (Widget|GetAllWidgetsOfClass "/Game/TwoLeftStanding/UI/WBP_PlayerHUD.WBP_PlayerHUD_C" true))
        (Widget|SetVisibility (Variables|/Game/TwoLeftStanding/UI/WBP_PlayerHUD.WBP_PlayerHUD_C|GetImg_Crosshair (Utilities|Array|Get(acopy) _foundwidgets)) "SelfHitTestInvisible")
        (else
          (bind _returnvalue_3 (UserInterface|CreateWidget "/Game/TwoLeftStanding/UI/WBP_LevelSelect.WBP_LevelSelect_C"))
          (bind _output_get (Variables|Default|SetLevelSelectUIRef _returnvalue_3))
          (UserInterface|Viewport|AddtoViewport _output_get 0)
          (Variables|Default|SetbIsMenuOpen true)
          (Variables|/Script/Engine.PlayerController|SetbShowMouseCursor _returnvalue_2 true)
          (Input|SetInputModeGameandUI _returnvalue_2 _returnvalue_3 "DoNotLock" true false)
          (bind _foundwidgets_2 (Widget|GetAllWidgetsOfClass "/Game/TwoLeftStanding/UI/WBP_PlayerHUD.WBP_PlayerHUD_C" true))
          (Widget|SetVisibility (Variables|/Game/TwoLeftStanding/UI/WBP_PlayerHUD.WBP_PlayerHUD_C|GetImg_Crosshair (Utilities|Array|Get(acopy) _foundwidgets_2)) "Hidden"))))))

(fn ConstructionScript)

(fn OnRepModelIndex
  (CallFunction|UpdateCharacterModel))

(fn UpdateCharacterModel
  (bind _mesh (Variables|Character|GetMesh))
  (Components|SkeletalMesh|SetSkeletalMeshAsset _mesh (Utilities|Select :Index (Variables|Default|GetModelIndex) :Option%200 "/Game/TwoLeftStanding/Player/Characters/starlord/starlord_rest_pose.starlord_rest_pose" :Option%201 "/Game/TwoLeftStanding/Player/Characters/psylocke/Psylocke_Fleet_Butterfly_rest_pose.Psylocke_Fleet_Butterfly_rest_pose"))
  (Components|SkeletalMesh|SetAnimInstanceClass _mesh (Utilities|Select :Index (Variables|Default|GetModelIndex) :Option%200 "/Game/TwoLeftStanding/Player/ABP_Male.ABP_Male_C" :Option%201 "/Game/TwoLeftStanding/Player/ABP_Female.ABP_Female_C"))
  (Rendering|Material|SetMaterial (Variables|Default|GetGunMesh) 0 (Utilities|Select :Index (Variables|Default|GetModelIndex) :Option%200 "/Game/TwoLeftStanding/Player/Weapon/SciFiGun_Blue/scifigun_blue.scifigun_blue" :Option%201 "/Game/TwoLeftStanding/Player/Weapon/SciFiGun_Purple/scifigun_purple.scifigun_purple")))