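; Player controller for the main menu that shows WBP_MainMenu with a mouse cursor and connects to Photon on BeginPlay.
; Hosting creates a Photon Fusion room, then flags the GameInstance as lobby host and creates a two-player advanced session tagged with the room name.
; Fetching sessions rebuilds the menu's session list from advanced-session search results, while quick join and specific join go through Photon random or named room joins.
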(event Custom|ExecuteFusionHost
  (params (RoomName :type String))
  (|Room (Utilities|Struct|MakeFusionRoomOptions RoomName 0 5 2 true true "/Game/TwoLeftStanding/Maps/Map_Lobby.Map_Lobby")
    (:OnFailure
      (Development|PrintString "Host Failed: Check App ID or Connection."))
    (:OnSuccess
      (Development|PrintString "Host Successful! Loading Map...")
      (bind _asbp_two_left_game_instance (Utilities|Casting|CastToBP_TwoLeftGameInstance (Game|GetGameInstance)))
      (Variables|/Game/TwoLeftStanding/BP_TwoLeftGameInstance.BP_TwoLeftGameInstance_C|SetbIsLobbyHost _asbp_two_left_game_instance true)
      (|AdvancedSession (Utilities|Array|MakeArray (Class|AdvancedSessionsLibrary|MakeLiteralSessionPropertyString "CustomRoomName" RoomName)) self 2 0 false true false true true false false false true false true))))

(event Custom|ExecuteFetchSessions
  (bind _results (|FindSessionsAdvanced self 20 false "AllServers" 0 false false false)
    (:OnSuccess
      (Widget|Panel|ClearChildren (Variables|/Game/TwoLeftStanding/UI/WBP_MainMenu.WBP_MainMenu_C|GetSb_SessionList (Variables|Default|GetMainMenuRef)))
      (for _array_element _results
        (bind _returnvalue (UserInterface|CreateWidget "/Game/TwoLeftStanding/UI/WBP_SessionRow.WBP_SessionRow_C" self _array_element))
        (Widget|Panel|AddChild (Variables|/Game/TwoLeftStanding/UI/WBP_MainMenu.WBP_MainMenu_C|GetSb_SessionList (Variables|Default|GetMainMenuRef)) _returnvalue)))))

(event Custom|ExecuteFusionQuickJoin
  (|JoinRandomRoom))

(event Custom|ExecuteSpecificJoin
  (params (RoomToJoin :type String))
  (|JoinRoom RoomToJoin))

(event EventBeginPlay
  (bind _returnvalue (Game|GetPlayerController 0))
  (bind _returnvalue_2 (UserInterface|CreateWidget "/Game/TwoLeftStanding/UI/WBP_MainMenu.WBP_MainMenu_C" _returnvalue))
  (Variables|Default|SetMainMenuRef _returnvalue_2)
  (UserInterface|Viewport|AddtoViewport _returnvalue_2 0)
  (Variables|/Script/Engine.PlayerController|SetbShowMouseCursor _returnvalue true)
  (Input|SetInputModeGameandUI _returnvalue _returnvalue_2 "DoNotLock" true false)
  (|ConnecttoPhoton))

(event EventTick
  (params (DeltaSeconds :type Float%20%28single-precision%29)))

(fn ConstructionScript)