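; BP_ExitZone is a multiplayer extraction zone that completes the level when it is active and holds two players.
; Multicast_ActivateExit activates the exit and turns its status light green.
; The server counts players via ExtractionZone overlaps and checks for completion both on entry and on activation, covering players already inside.
; On completion it pauses the game and calls ClientShowLevelComplete on every BP_TwoLeftPlayer.
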(event OnComponentBeginOverlap(ExtractionZone)
  (params (OverlappedComponent :type Primitive%20Component%20Object%20Reference) (OtherActor :type Actor%20Object%20Reference) (OtherComp :type Primitive%20Component%20Object%20Reference) (OtherBodyIndex :type Integer) (bFromSweep :type Boolean) (SweepResult :type Hit%20Result%20Structure%20%28by%20ref%29))
  (Networking|SwitchHasAuthority
    (:Authority
      (Utilities|Casting|CastToTwoLeftPlayer OtherActor)
      (bind _result (Math|Integer|IncrementInt (Variables|Default|GetPlayersInZone))
        (:%20%20
          (Variables|Default|SetPlayersInZone _result)
          (if (and (Variables|Default|GetbIsActive) (== (Variables|Default|GetPlayersInZone) 2))
            (Development|PrintString "Level Completed!")
            (Game|SetGamePaused true)
            (bind _outactors (Actor|GetAllActorsOfClass "/Game/TwoLeftStanding/Player/BP_TwoLeftPlayer.BP_TwoLeftPlayer_C"))
            (for _array_element _outactors
              (Default|ClientShowLevelComplete _array_element))))))))

(event OnComponentEndOverlap(ExtractionZone)
  (params (OverlappedComponent :type Primitive%20Component%20Object%20Reference) (OtherActor :type Actor%20Object%20Reference) (OtherComp :type Primitive%20Component%20Object%20Reference) (OtherBodyIndex :type Integer))
  (Networking|SwitchHasAuthority
    (:Authority
      (Utilities|Casting|CastToTwoLeftPlayer OtherActor)
      (bind _result (Math|Integer|DecrementInt (Variables|Default|GetPlayersInZone))
        (:%20%20
          (Variables|Default|SetPlayersInZone _result))))))

(event Custom|Multicast_ActivateExit
  (Variables|Default|SetbIsActive true)
  (Rendering|Components|Light|SetLightColor (Variables|Default|GetStatusLight) "(R=0.120194,G=1.000000,B=0.000000,A=1.000000)" true)
  (Networking|SwitchHasAuthority
    (:Authority
      (if (== (Variables|Default|GetPlayersInZone) 2)
        (Development|PrintString "Level Completed!")
        (Game|SetGamePaused true)
        (bind _outactors (Actor|GetAllActorsOfClass "/Game/TwoLeftStanding/Player/BP_TwoLeftPlayer.BP_TwoLeftPlayer_C"))
        (for _array_element _outactors
          (Default|ClientShowLevelComplete _array_element))))))

(event EventBeginPlay)

(event Collision|EventActorBeginOverlap
  (params (OtherActor :type Actor%20Object%20Reference)))

(event EventTick
  (params (DeltaSeconds :type Float%20%28single-precision%29)))

(fn ConstructionScript)