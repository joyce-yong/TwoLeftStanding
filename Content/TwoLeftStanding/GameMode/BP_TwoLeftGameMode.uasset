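; Game mode for TwoLeftStanding, a two-player co-op level with a kill quota and an escape objective.
; A looping timer checks whether both players are dead, then pauses the game, multicasts their dissolve and, after a Delay, calls the level-failed screen on clients.
; AddTeamKill counts shared kills and, at quota, activates BP_ExitZone and updates each controller's objective UI.
; ChoosePlayerStart assigns PlayerStarts round-robin through an incrementing index.
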(event Custom|CheckGameOver
  (bind _outactors (Actor|GetAllActorsOfClass "/Game/TwoLeftStanding/Player/BP_TwoLeftPlayer.BP_TwoLeftPlayer_C"))
  (if (== (Utilities|Array|Length _outactors) 2)
    (if (and (Variables|/Script/TwoLeftStanding.TwoLeftPlayer|GetbIsDead (Utilities|Array|Get(acopy) _outactors)) (Variables|/Script/TwoLeftStanding.TwoLeftPlayer|GetbIsDead (Utilities|Array|Get(acopy) _outactors 1)))
      (Utilities|Time|ClearandInvalidateTimerbyHandle (Variables|Default|GetGameOverTimer))
      (Game|SetGamePaused true)
      (bind _outactors_2 (Actor|GetAllActorsOfClass "/Game/TwoLeftStanding/Player/BP_TwoLeftPlayer.BP_TwoLeftPlayer_C"))
      (for _array_element _outactors_2
        (Class|TwoLeftPlayer|MulticastStartDissolve _array_element))
      (Utilities|FlowControl|Delay 3.0)
      (bind _outactors_3 (Actor|GetAllActorsOfClass "/Game/TwoLeftStanding/Player/BP_TwoLeftPlayer.BP_TwoLeftPlayer_C"))
      (for _array_element_2 _outactors_3
        (Default|ClientShowLevelFailed _array_element_2)))))

(event Custom|AddTeamKill
  (bind _result (Math|Integer|IncrementInt (Variables|Default|GetCurrentTeamKills))
    (:%20%20
      (if (>= _result (Variables|Default|GetRequiredKills))
        (Development|PrintString "Quota Reached! Exit Zone Unlocked!")
        (bind _returnvalue (Actor|GetActorOfClass "/Game/TwoLeftStanding/BP_ExitZone.BP_ExitZone_C"))
        (Default|MulticastActivateExit _returnvalue)
        (bind _outactors (Actor|GetAllActorsOfClass "/Game/TwoLeftStanding/BP_TwoLeftController.BP_TwoLeftController_C"))
        (for _array_element _outactors
          (Default|ClientUpdateObjectiveUI _array_element "The Exit Zone is Unlocked! Escape Now!"))))))

(event EventBeginPlay
  (bind _returnvalue (Utilities|Time|SetTimerbyEvent (delegate Custom|CheckGameOver) 0.5 true))
  (Variables|Default|SetGameOverTimer _returnvalue))

(event EventTick
  (params (DeltaSeconds :type Float%20%28single-precision%29)))

(fn ConstructionScript)

(fn ChoosePlayerStart
  (params (Player :type Controller%20Object%20Reference))
  (bind _outactors (Actor|GetAllActorsOfClass "/Script/Engine.PlayerStart"))
  (Variables|Default|SetSpawnIndex (+ (Variables|Default|GetSpawnIndex) 1))
  (return (Utilities|Array|Get(acopy) _outactors (Math|Integer|%(Integer) (Variables|Default|GetSpawnIndex) (Utilities|Array|Length _outactors)))))